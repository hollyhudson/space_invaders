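; Ball actor Blueprint with a sketched bounce model, mostly unwired.
; Custom events compute a new velocity by negating one axis of the current one, with the Y and Z reversals also subtracting gravity from X.
; Unconnected nodes would derive room boundaries from the Vive pawn's wall locations and fixed limits, or boost the ball's physics velocity.
; BeginPlay and Hit are empty, and nothing here calls the reversals or applies their result.
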(event `self.ReceiveBeginPlay`
  ;[1 1 1] get right and left wall boundaries
)

(event `Reverse X Velocity`
  ;[1 1 1] Comment
  (set `self.new_velocity` (`KismetMathLibrary.MakeVector` (* (.x (`self.current_velocity`)) -1.0) (.y (`self.current_velocity`)) (.z (`self.current_velocity`)))))

(event `Reverse Y Velocity`
  ;[1 1 1] Comment
  (set `self.new_velocity` (`KismetMathLibrary.MakeVector` (- (.x (`self.current_velocity`)) (`self.gravity`)) (* (.y (`self.current_velocity`)) -1.0) (.z (`self.current_velocity`)))))

(event `Reverse Z Velocity`
  ;[1 1 1] Comment
  (set `self.new_velocity` (`KismetMathLibrary.MakeVector` (- (.x (`self.current_velocity`)) (`self.gravity`)) (.y (`self.current_velocity`)) (* (.z (`self.current_velocity`)) -1.0))))

(event `self.ReceiveHit`
  (params (MyComp :type "PrimitiveComponent Object Reference") (Other :type "Actor Object Reference") (OtherComp :type "PrimitiveComponent Object Reference") (bSelfMoved :type Boolean) (HitLocation :type "Vector Structure") (HitNormal :type "Vector Structure") (NormalImpulse :type "Vector Structure") (Hit :type "HitResult Structure (by ref)")))

(fn `UserConstructionScript`)