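; City mids Blueprint that procedurally lays out a block of static meshes, apparently mid-size city buildings, in a square grid.
; The construction script uses nested loops to add evenly spaced mesh components, each with a random quarter-turn yaw that rerolls whenever the script reruns.
; A random floor-stacking loop is left disconnected, so each cell gets a single mesh, and the event graph holds only disabled stubs.
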(fn `UserConstructionScript`
  (for _index (range 5)
    (for _index_2 (range 5)
      (`AddComponent|NODE_AddStaticMeshComponent-0` :`RelativeTransform` (`KismetMathLibrary.MakeTransform` (`KismetMathLibrary.MakeVector` (`KismetMathLibrary.Conv_IntToDouble` (* _index_2 5000)) (`KismetMathLibrary.Conv_IntToDouble` (* _index 5000))) (`KismetMathLibrary.MakeRotator` 0.0 0.0 (`KismetMathLibrary.Conv_IntToDouble` (* (`KismetMathLibrary.RandomIntegerInRange` 0 3) 90))))))))